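; Stamina component that tracks its owner's current stamina and regenerates it over time.
; A looping timer feeds AddStamina, which clamps the value, sends the normalized result to the owner through an interface message, and fires dispatchers when stamina is low or empty.
; StopRegen pauses that timer and, given a positive duration, schedules a one-shot timer to resume it, replacing any pending restart.
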(event Custom|StaminaRegeneration
  (CallFunction|AddStamina (* (Variables|Default|GetStaminaRegenPerSecond) (Variables|Default|GetStaminaRegenInterval))))

(event Custom|StopRegen
  (params (StopTime :type Float%20%28single-precision%29))
  (Utilities|Time|ClearandInvalidateTimerbyHandle (Variables|Default|GetRestartRegenTimerRef))
  (Utilities|Time|PauseTimerbyHandle (Variables|Default|GetTimerRef))
  (if (> StopTime 0.0)
    (bind _returnvalue (Utilities|Time|SetTimerbyEvent (delegate Custom|RestartRegen) StopTime))
    (Variables|Default|SetRestartRegenTimerRef _returnvalue)))

(event Custom|RestartRegen
  (Utilities|Time|UnpauseTimerbyHandle (Variables|Default|GetTimerRef)))

(event EventBeginPlay
  (Variables|Default|SetCurrentStamina (Variables|Default|GetMaxStamina))
  (bind _returnvalue (Utilities|Time|SetTimerbyEvent (delegate Custom|StaminaRegeneration) (Variables|Default|GetStaminaRegenInterval) true))
  (Variables|Default|SetTimerRef _returnvalue))

(fn AddStamina
  (params (StaminaChange :type Float%20%28single-precision%29))
  (bind _output_get (Variables|Default|SetCurrentStamina (Math|Float|Clamp(Float) (+ StaminaChange (Variables|Default|GetCurrentStamina)) 0.0 (Variables|Default|GetMaxStamina))))
  (Class|BPIStaminaCommunication|SetStaminaValue(Message) (Components|GetOwner) (/ _output_get (Variables|Default|GetMaxStamina)))
  (if (<= (Variables|Default|GetCurrentStamina) 0.0)
    (Default|CallOutOfStamina)
    (elif (<= (/ _output_get (Variables|Default|GetMaxStamina)) 0.25)
      (Default|CallLowAmountOfStamina)))
  (return))